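; Test Blueprint that drives procedural chunked terrain generation with levels of detail around an observed object.
; BeginPlay initializes the system with the Bp_observedObject actor and passes in chunk, noise, height, UV and LOD settings, deriving max LOD from the LodRepetitions count.
; Tick refreshes data and requests generation of possible data, while a fast looping timer separately asks to display chunks, decoupling display updates from generation.
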(event Custom|RefreshChunks
  (Class|TerrainGenerator|AsktoDisplayChunks))

(event EventBeginPlay
  (bind _returnvalue (Actor|GetActorOfClass "/Game/bp_observedObject.bp_observedObject_C"))
  (Initialization|Initialize _returnvalue)
  (Class|ChunkFunctionLibrary|SetTerrainGenerationSettings (Variables|Default|GetChunk%20Width) (Variables|Default|GetNoise%20Scale) (Variables|Default|GetHeight%20Multiplier) (Variables|Default|GetUVScale) (Math|Conversions|ToByte(Integer) (- (Utilities|Array|Length (Variables|Default|GetlodRepetitions)) 1)))
  (Utilities|Time|SetTimerbyEvent (delegate Custom|RefreshChunks) 0.1 true))

(event EventTick
  (params (DeltaSeconds :type Float%20%28single-precision%29))
  (Class|TerrainGenerator|RefreshDatas)
  (Class|TerrainGenerator|AsktoGeneratePossibleData))

(fn ConstructionScript)